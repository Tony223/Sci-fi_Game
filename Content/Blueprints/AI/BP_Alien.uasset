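; Enemy alien character that chases the player marine, melee-attacks in range and shows a health bar.
; A repeating AIMoveTo drives the chase, while Tick updates the bar and plays the attack montage with movement paused.
; DamagePlayer applies hit damage but is not called within this Blueprint.
; Lethal damage disables movement and collision, credits the marine's kill, notifies the GameMode and destroys the alien after a delay.
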(event `self.ReceiveBeginPlay`
  (bind _asbp_marine (cast `/Game/Blueprints/Characters/BP_Marine` (`GameplayStatics.GetPlayerPawn` 0)))
  (set `self.Marine` _asbp_marine)
  (bind _aswbp_alien_health_bar (cast `/Game/UI/WBP_AlienHealthBar` (`WidgetComponent.GetUserWidgetObject` (`self.Widget`))))
  (set `self.HealthBar` _aswbp_alien_health_bar)
  (if (`self.IsAlive`)
    (`|AIMoveTo` self (0.0 0.0 0.0) (`self.Marine`) :!label _label
      (:`OnSuccess`
        _)
      (:`OnFail`
        _))
    (`KismetSystemLibrary.Delay` 0.2)
    (goto _label)))

(event `self.ReceiveTick`
  (params (DeltaSeconds :type "Float (single-precision)"))
  (set `/Game/UI/WBP_AlienHealthBar.Health` (`self.Health`) (`self.HealthBar`))
  (if (`self.CanAttack`)
    (`self.DeactivateAIMovement`)
    (`|PlayMontage` (`self.Mesh`) "/Game/Characters/Enemy_Great_Spider/Animations/AM_AlienAttack.AM_AlienAttack"
      (:`OnCompleted`
        (`self.ActivateAIMovement`)))))

(event `self.ReceiveAnyDamage`
  (params (Damage :type "Float (single-precision)") (DamageType :type "DamageType Object Reference") (InstigatedBy :type "Controller Object Reference") (DamageCauser :type "Actor Object Reference"))
  (bind _returnvalue (`self.TakeDamage` Damage))
  (if _returnvalue
    (`self.KillAlien`)
    (`KismetSystemLibrary.Delay` 3.0)
    (`self.K2_DestroyActor`)))

(fn `ActivateAIMovement`
  (`ActorComponent.Activate` (`self.CharacterMovement`) false))

(fn `CanAttack`
  (returns (ReturnValue :type Boolean))
  (return (and (`self.Is Within Attack Range`) (not (`self.IsAttacking`)) (`self.IsAlive`) (`self.IsAlive` (`self.Marine`)))))

(fn `DamagePlayer`
  (`GameplayStatics.ApplyDamage` (`GameplayStatics.GetPlayerPawn` 0) (`self.DamagePerHit`)))

(fn `DeactivateAIMovement`
  (`ActorComponent.Deactivate` (`self.CharacterMovement`)))

(fn `Is Within Attack Range`
  (returns (ReturnValue :type Boolean))
  (return (< (`self.GetDistanceTo` (`GameplayStatics.GetPlayerPawn` 0)) (`self.AttackRange`))))

(fn `IsAttacking`
  (returns (ReturnValue :type Boolean))
  (return (`AnimInstance.Montage_IsPlaying` (`SkeletalMeshComponent.GetAnimInstance` (`self.Mesh`)) "/Game/Characters/Enemy_Great_Spider/Animations/AM_AlienAttack.AM_AlienAttack")))

(fn `KillAlien`
  (set `self.IsDead` true)
  (`self.DeactivateAIMovement`)
  (`self.SetActorEnableCollision` false)
  (bind _asbp_marine (cast `/Game/Blueprints/Characters/BP_Marine` (`GameplayStatics.GetPlayerPawn` 0)))
  (`/Game/Blueprints/Characters/BP_Marine.IncreaseKills` _asbp_marine)
  (bind _asbp_game_mode (cast `/Game/Blueprints/GameModes/BP_GameMode` (`GameplayStatics.GetGameMode`)))
  (`/Game/Blueprints/GameModes/BP_GameMode.RegisterAlienDeath` _asbp_game_mode self)
  (`ActorComponent.K2_DestroyComponent` (`self.Widget`)))

(fn `UserConstructionScript`)