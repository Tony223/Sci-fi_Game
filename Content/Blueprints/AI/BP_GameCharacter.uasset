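; BP_GameCharacter is an AI-folder character Blueprint that provides basic health and damage handling.
; TakeDamage applies damage only while IsAlive, then returns whether the clamped Health from DecreaseHealth has reached zero.
; IsAlive simply negates the IsDead flag, which none of these functions set, so reaching zero health does not itself mark the character dead here.
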(fn `DecreaseHealth`
  (params (DamageAmount :type "Float (double-precision)"))
  (returns (Health :type "Float (double-precision)"))
  (bind _output_get (set `self.Health` (`KismetMathLibrary.FClamp` (- (`self.Health`) DamageAmount) 0.0 100.0)))
  (return _output_get))

(fn `IsAlive`
  (returns (ReturnValue :type Boolean))
  (return (not (`self.IsDead`))))

(fn `TakeDamage`
  (params (DamageAmount :type "Float (double-precision)"))
  (returns (ReturnValue :type Boolean))
  (if (`self.IsAlive`)
    (bind _health (`self.DecreaseHealth` DamageAmount))
    (return (== _health 0.0))))

(fn `UserConstructionScript`)