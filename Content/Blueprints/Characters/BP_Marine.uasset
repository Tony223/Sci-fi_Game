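; Player-controlled marine for a cursor-aimed shooter, with world-axis movement, a HUD, health pickup helpers and a kill counter.
; While alive, it smoothly turns control rotation toward the point under the mouse each tick.
; Firing loops sound and muzzle particles while a timer repeats line traces from the muzzle along actor forward, applying damage and impact effects.
; MovementButaforia and Dich are empty functions holding unreachable copies of event logic.
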(event `self.ReceiveBeginPlay`
  (bind _output_get (set `self.PlayerController` (`GameplayStatics.GetPlayerController` 0)))
  (set `PlayerController.bShowMouseCursor` true _output_get)
  (bind _returnvalue (`|CreateWidget` "/Game/UI/WBP_PlayerHUD.WBP_PlayerHUD_C" null self))
  (`UserWidget.AddToViewport` _returnvalue 0))

(event `self.ReceiveTick`
  (params (DeltaSeconds :type "Float (single-precision)"))
  (if (`self.IsAlive`)
    (`self.UpdatePlayerAim` DeltaSeconds)))

(event `InputAxis|MoveForward`
  (params (AxisValue :type "Float (single-precision)"))
  (if (`self.IsAlive`)
    (`self.AddMovementInput` (1.0 0.0 0.0) AxisValue)))

(event `InputAxis|MoveRight`
  (params (AxisValue :type "Float (single-precision)"))
  (if (`self.IsAlive`)
    (`self.AddMovementInput` (0.0 1.0 0.0) AxisValue)))

(event `self.ReceiveAnyDamage`
  (params (Damage :type "Float (single-precision)") (DamageType :type "DamageType Object Reference") (InstigatedBy :type "Controller Object Reference") (DamageCauser :type "Actor Object Reference"))
  (bind _returnvalue (`self.TakeDamage` Damage))
  (if _returnvalue
    (set `self.IsDead` true)
    (`self.StopFiring`)))

(event `InputAction|Fire`
  (params (Key :type "Key Structure"))
  (:`Pressed`
    (`self.StartFiring`))
  (:`Released`
    (`self.StopFiring`)))

(fn `AddHealth`
  (params (HealthToAdd :type "Float (double-precision)"))
  (set `self.Health` (`KismetMathLibrary.FClamp` (+ (`self.Health`) HealthToAdd) 0.0 100.0)))

(fn `dich`)

(fn `GetWeaponTraceEndLocation`
  (returns (ReturnValue :type "Vector Structure"))
  (return (+ (`self.GetWeaponTraceStartLocation`) (* (`self.GetActorForwardVector`) (`self.WeaponRange`)))))

(fn `GetWeaponTraceStartLocation`
  (returns (ReturnValue :type "Vector Structure"))
  (return (`SceneComponent.GetSocketLocation` (`self.Rifle`) "MuzzleFlash")))

(fn `IncreaseKills`
  (`/Engine/EditorBlueprintResources/StandardMacros.IncrementInt` (`self.Kills`)))

(fn `IsHealthFull`
  (returns (ReturnValue :type Boolean))
  (return (== (`self.Health`) 100.0)))

(fn `MovementButaforia`)

(fn `SpawnImpactHit`
  (params (HitLocation :type "Vector Structure"))
  (`GameplayStatics.SpawnEmitterAtLocation` "/Game/Effects/Weapons/Impacts/P_AssaultRifle_IH.P_AssaultRifle_IH" HitLocation))

(fn `StartFiring`
  (if (`self.IsAlive`)
    (`ActorComponent.Activate` (`self.P_AssaultRifle_MF`) false)
    (bind _returnvalue (`GameplayStatics.SpawnSound2D` "/Game/Sounds/Weapon_AssaultRifle/Stereo/A_RifleFireLoop_Cue.A_RifleFireLoop_Cue" 1.0 1.0 0.0 null))
    (set `self.RifleFireSound` _returnvalue)
    (`self.WeaponTrace`)
    (`KismetSystemLibrary.K2_SetTimer` null "WeaponTrace" (`self.WeaponFireRate`) true)))

(fn `StopFiring`
  (bind _riflefiresound (`self.RifleFireSound`))
  (`ActorComponent.Deactivate` (`self.P_AssaultRifle_MF`))
  (`/Engine/EditorBlueprintResources/StandardMacros.IsValid` _riflefiresound
    (:`Is Valid`
      (`AudioComponent.Stop` _riflefiresound)
      (`GameplayStatics.SpawnSound2D` "/Game/Sounds/Weapon_AssaultRifle/Stereo/A_RifleFireEnd_Cue.A_RifleFireEnd_Cue" 1.0 1.0 0.0 null)
      (`KismetSystemLibrary.K2_ClearTimer` null "WeaponTrace"))))

(fn `UpdatePlayerAim`
  (params (DeltaTime :type "Float (double-precision)"))
  (`/Engine/EditorBlueprintResources/StandardMacros.IsValid` (`self.PlayerController`)
    (:`Is Valid`
      (`Controller.SetControlRotation` (`self.PlayerController`) (`KismetMathLibrary.RInterpTo` (`Controller.GetControlRotation` (`self.PlayerController`)) (`KismetMathLibrary.FindLookAtRotation` (`self.K2_GetActorLocation`) (`.Location` (`GameplayStatics.BreakHitResult` (`PlayerController.GetHitResultUnderCursorByChannel` (`self.PlayerController`) "TraceTypeQuery1" true)))) (`local.DeltaTime`) (`self.InterpSpeed`))))))

(fn `UserConstructionScript`)

(fn `WeaponTrace`
  (bind _outhit (`KismetSystemLibrary.LineTraceSingle` (`self.GetWeaponTraceStartLocation`) (`self.GetWeaponTraceEndLocation`) "TraceTypeQuery2"))
  (if (`GameplayStatics.BreakHitResult` _outhit)
    (`GameplayStatics.ApplyDamage` (`.HitActor` (`GameplayStatics.BreakHitResult` _outhit)) (`self.DamagePerShot`))
    (`self.SpawnImpactHit` (`.Location` (`GameplayStatics.BreakHitResult` _outhit)))))